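; LeftDoorTony is an enemy Blueprint that advances Tony through numbered rooms on randomly timed movement opportunities, with odds set by Difficulty.
; From BeginPlay, a looping event waits a few seconds, then rolls between Difficulty and 20, succeeding only on the minimum.
; A success increments CurrentRoom and calls CallMoveLeftTony, unless RecentlyMoved is set.
; That flag blocks back-to-back moves, clearing on a failed roll or after a short delay.
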(event Custom|MovementOpportunity
  (Utilities|FlowControl|RetriggerableDelay (Math|Random|RandomFloatinRange 3.0 5.0) :!label _label)
  (if (<= (Math|Random|RandomIntegerinRange (Variables|Default|GetDifficulty) 20) (Variables|Default|GetDifficulty))
    (if (not (Variables|Default|GetRecentlyMoved?))
      (Variables|Default|SetCurrentRoom (+ (Variables|Default|GetCurrentRoom) 1))
      (Default|CallMoveLeftTony)
      (Variables|Default|SetRecentlyMoved? true)
      (goto _label)
      (else
        (Utilities|FlowControl|Delay 2.5)
        (Variables|Default|SetRecentlyMoved? false)
        (goto _label)))
    (else
      (Variables|Default|SetRecentlyMoved? false)
      (goto _label))))

(event EventBeginPlay
  (CallFunction|MovementOpportunity))

(event Collision|EventActorBeginOverlap
  (params (OtherActor :type Actor%20Object%20Reference)))

(event EventTick
  (params (DeltaSeconds :type Float%20%28single-precision%29)))

(fn ConstructionScript)